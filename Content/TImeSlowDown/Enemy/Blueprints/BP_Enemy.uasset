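; BP_Enemy is an enemy that chases the ThirdPersonCharacter and can be individually slowed in time.
; PawnSensing triggers an AI MoveTo toward any ThirdPersonCharacter it sees.
; The ActivaeSlowMo event lowers the enemy's own CustomTimeDilation, then restores normal speed after a delay.
; BeginPlay caches the first ThirdPersonCharacter in the level, though the graph shown never reads that reference.
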(event `self.ReceiveBeginPlay`
  (bind _outactors (`GameplayStatics.GetAllActorsOfClass` "/Game/ThirdPersonBP/Blueprints/ThirdPersonCharacter.ThirdPersonCharacter_C"))
  (set `self.CharacterRefrence` (`|GetArrayItem` _outactors)))

(event `ActivaeSlowMo`
  (set `self.CustomTimeDilation` 0.3)
  (`KismetSystemLibrary.Delay` 4.0)
  (set `self.CustomTimeDilation` 1.0))

(event `self.PawnSensing.OnSeePawn`
  (params (Pawn :type "Pawn Object Reference"))
  (bind _asthird_person_character (cast `/Game/ThirdPersonBP/Blueprints/ThirdPersonCharacter` Pawn))
  (`|AIMoveTo` self (0.0 0.0 0.0) _asthird_person_character))

(fn `UserConstructionScript`)