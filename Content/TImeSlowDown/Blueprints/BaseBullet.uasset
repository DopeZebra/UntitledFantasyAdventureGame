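; BaseBullet is a projectile Blueprint in the TImeSlowDown folder that lives for one second after spawning.
; On BeginPlay it caches the first ThirdPersonCharacter found in the level.
; Its first hit prints the other actor's name and, if that actor is a BP_Enemy, calls DamageNormalArrowsMessage on the cached character rather than damaging the enemy directly.
; A CallDoDamage call is present but never runs.
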(event `self.ReceiveBeginPlay`
  (bind _outactors (`GameplayStatics.GetAllActorsOfClass` "/Game/ThirdPersonBP/Blueprints/ThirdPersonCharacter.ThirdPersonCharacter_C"))
  (set `self.CharacterREfrence` (`|GetArrayItem` _outactors))
  (`self.SetLifeSpan` 1.0))

(event `self.Hit`
  (params (`Hit Component` :type "PrimitiveComponent Object Reference") (`Other Actor` :type "Actor Object Reference"))
  (`/Engine/EditorBlueprintResources/StandardMacros.DoOnce` false
    (:`Completed`
      (`KismetSystemLibrary.PrintString` (`KismetSystemLibrary.GetDisplayName` `Other Actor`))
      (cast `/Game/TImeSlowDown/Enemy/Blueprints/BP_Enemy` `Other Actor`)
      (message `/Game/TImeSlowDown/Enemy/Blueprints/DamageInterface.DamageNormalArrows` (`self.CharacterREfrence`))
      (`KismetSystemLibrary.PrintString` "normal"))))

(fn `UserConstructionScript`
  (`parent.UserConstructionScript`))