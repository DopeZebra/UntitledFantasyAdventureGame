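; AI controller for the patrolling enemy pawn, BP_PetrolEnemy.
; On BeginPlay it runs the PetrolEnemy_BT behavior tree, then casts and caches the controlled pawn.
; It seeds the blackboard from the pawn's PathPetrol settings, copying the looping flag and wait time, and sets an initial forward Direction for the tree to use.
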(event `self.ReceiveBeginPlay`
  (`self.RunBehaviorTree` "/Game/TImeSlowDown/AI/BehaviorTree/PetrolEnemy_BT.PetrolEnemy_BT")
  (bind _asbp_petrol_enemy (cast `/Game/TImeSlowDown/AI/Blueprints/BP_PetrolEnemy` (`self.K2_GetPawn`)))
  (bind _output_get (set `self.PertolEnemyRefrence` _asbp_petrol_enemy))
  (`BlackboardComponent.SetValueAsBool` (`AIBlueprintHelperLibrary.GetBlackboard` null) "PathLooping" (`/Game/TImeSlowDown/AI/Blueprints/PetrolPath.IsLooping` (`/Game/TImeSlowDown/AI/Blueprints/BP_PetrolEnemy.PathPetrol` _output_get)))
  (`BlackboardComponent.SetValueAsInt` (`AIBlueprintHelperLibrary.GetBlackboard` null) "Direction" 1)
  (`BlackboardComponent.SetValueAsFloat` (`AIBlueprintHelperLibrary.GetBlackboard` null) "WaitTime" (`/Game/TImeSlowDown/AI/Blueprints/PetrolPath.WaitTime` (`/Game/TImeSlowDown/AI/Blueprints/BP_PetrolEnemy.PathPetrol` (`self.PertolEnemyRefrence`)))))

(fn `UserConstructionScript`)