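; AI controller for Enemy1 that runs its behavior tree and feeds it patrol and perception state.
; On BeginPlay it starts Enemy1_BT, then copies the controlled enemy's patrol path looping flag and wait time to the blackboard and sets an initial direction.
; Perception updates for the third-person character write CanSeePlayer from whether the stimulus was successfully sensed.
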(event `self.ReceiveBeginPlay`
  (`self.RunBehaviorTree` "/Game/TImeSlowDown/AI/Enemy1_BT.Enemy1_BT")
  (bind _asbp_aienemy_1 (cast `/Game/TImeSlowDown/AI/Blueprints/BP_AIEnemy1` (`self.K2_GetPawn`)))
  (bind _output_get (set `self.EnemyRefrence` _asbp_aienemy_1))
  (`BlackboardComponent.SetValueAsBool` (`AIBlueprintHelperLibrary.GetBlackboard` null) "PathLooping" (`/Game/TImeSlowDown/AI/Blueprints/PetrolPath.IsLooping` (`/Game/TImeSlowDown/AI/Blueprints/BP_AIEnemy1.PetrolPath` _output_get)))
  (`BlackboardComponent.SetValueAsInt` (`AIBlueprintHelperLibrary.GetBlackboard` null) "Direction" 1)
  (`BlackboardComponent.SetValueAsFloat` (`AIBlueprintHelperLibrary.GetBlackboard` null) "WaitTime" (`/Game/TImeSlowDown/AI/Blueprints/PetrolPath.WaitTime` (`/Game/TImeSlowDown/AI/Blueprints/BP_AIEnemy1.PetrolPath` (`self.EnemyRefrence`)))))

(event `self.AIPerception.OnTargetPerceptionUpdated`
  (params (Actor :type "Actor Object Reference") (Stimulus :type "AIStimulus Structure"))
  (cast `/Game/ThirdPersonBP/Blueprints/ThirdPersonCharacter` Actor)
  (`BlackboardComponent.SetValueAsBool` (`AIBlueprintHelperLibrary.GetBlackboard` null) "CanSeePlayer" (`.bSuccessfullySensed` (break `AIStimulus` Stimulus))))

(fn `UserConstructionScript`)