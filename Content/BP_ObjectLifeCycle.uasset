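; Actor that cycles a static mesh through an array of stage meshes when F is pressed, animating a material transition between stages.
; BeginPlay creates a dynamic material instance per stage, while the construction script previews the mesh at StartIndex.
; A timeline drives "Amount Of Change" on the outgoing material, then the index advances with wraparound and a second timeline animates the new one.
; A DoOnce blocks input until the transition finishes.
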(event `self.ReceiveBeginPlay`
  (`|ExecutionSequence`
    (:`then_0`
      ;[0 0.8359 1] Create Dynamic Material Istance
      (for _array_element (`self.Stages Of Actor`)
        (bind _returnvalue (`PrimitiveComponent.CreateDynamicMaterialInstance` (`self.StaticMeshComponent`) 0 (`StaticMesh.GetMaterial` _array_element 0) "None"))
        (`KismetArrayLibrary.Array_Add` (`self.Stages Of Actor Materials`) _returnvalue))
      (`self.Set Mesh And Material` (`self.Start Index`)))
    (:`then_1`
      (set `self.CurrentIndex` (`self.Start Index`)))
    (:`then_2`
      (for _array_element_2 (`self.Stages Of Actor Materials`)
        (if (not (== (`PrimitiveComponent.GetMaterial` (`self.StaticMeshComponent`) 0) _array_element_2))
          (`MaterialInstanceDynamic.SetScalarParameterValue` _array_element_2 "Amount Of Change" 0.0))))))

(event `Key|F`
  (params (Key :type "Key Structure"))
  (:`Pressed`
    (`/Engine/EditorBlueprintResources/StandardMacros.DoOnce` false :!label _label
      (:`Completed`
        (bind (_direction _decrease) (`Timeline|TransitionOutMesh` :!via `ReverseFromEnd`)
          (:`Update`
            (`MaterialInstanceDynamic.SetScalarParameterValue` (`|GetArrayItem` (`self.Stages Of Actor Materials`) (`self.CurrentIndex`)) "Amount Of Change" _decrease))
          (:`Finished`
            (bind _current_index (`self.Cycle Through Mesh`))
            (`self.Set Mesh And Material` _current_index)
            (bind (_direction_2 _increase) (`Timeline|TransitionInMesh` :!via `ReverseFromEnd`)
              (:`Update`
                (`MaterialInstanceDynamic.SetScalarParameterValue` (`|GetArrayItem` (`self.Stages Of Actor Materials`) (`self.CurrentIndex`)) "Amount Of Change" _increase))
              (:`Finished`
                (`self.Reset Do Once`)))))))))

(event `Reset Do Once`
  (goto _label :!via `Reset`))

(fn `Cycle Through Mesh`
  (returns (`Current Index` :type Integer))
  (bind _returnvalue (+ (`self.CurrentIndex`) 1))
  (`|ExecutionSequence`
    (:`then_0`
      (if (== _returnvalue (`KismetArrayLibrary.Array_Length` (`self.Stages Of Actor`)))
        (bind _output_get (set `self.CurrentIndex` 0))
        (else
          (set `self.CurrentIndex` _returnvalue)))
      (return _output_get))))

(fn `GetMesh`
  (returns (CurrentActor :type "StaticMesh Object Reference"))
  (return (`self.CurrentActor`)))

(fn `Set Mesh And Material`
  (params (Index :type Integer))
  (bind _staticmeshcomponent (`self.StaticMeshComponent`))
  (bind _output (`|GetArrayItem` (`self.Stages Of Actor`) Index))
  (`StaticMeshComponent.SetStaticMesh` _staticmeshcomponent _output)
  (`PrimitiveComponent.SetMaterial` _staticmeshcomponent 0 (`|GetArrayItem` (`self.Stages Of Actor Materials`) Index))
  (set `self.CurrentActor` _output))

(fn `UserConstructionScript`
  (`StaticMeshComponent.SetStaticMesh` (`self.StaticMeshComponent`) (`|GetArrayItem` (`self.Stages Of Actor`) (`self.Start Index`))))