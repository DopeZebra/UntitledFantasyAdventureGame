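; BP_DamageDummy is a damageable test actor that tracks its health and is destroyed when that health fails a check.
; CurrentHealth starts at MaxHealth on BeginPlay.
; TakeDamage passes incoming damage through ReduceHealth, prints the new value for debugging, then runs HealthCheck to decide whether to call Dead, which destroys the actor.
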(event `self.ReceiveBeginPlay`
  (set `self.CurrentHealth` (`self.MaxHealth`)))

(event `/Game/Blueprints/Interface/DamageInterface_U.TakeDamage`
  (params (DamagedActor :type "Actor Object Reference") (DamageToApply :type "Float (single-precision)") (DamageCauser :type "Actor Object Reference"))
  (bind _output_get (set `self.CurrentHealth` (`/Game/Blueprints/CustomMacroLibraries/ML_HealthAndDamage.ReduceHealth` (`self.CurrentHealth`) DamageToApply)))
  (`KismetSystemLibrary.PrintString` (`KismetStringLibrary.Conv_DoubleToString` _output_get))
  (if (`/Game/Blueprints/CustomMacroLibraries/ML_HealthAndDamage.HealthCheck` _output_get)
    (`self.Dead`)))

(event `Dead`
  (`self.K2_DestroyActor`))

(fn `UserConstructionScript`)