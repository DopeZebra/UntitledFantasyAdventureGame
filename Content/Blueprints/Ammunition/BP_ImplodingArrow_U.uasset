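; Arrow projectile Blueprint that triggers an implode-and-explode effect on impact or after a short timeout.
; On CustomHit it plays a scaled-up lightning particle at the impact point, spawns BP_ImplodeAndExplode at its own transform, flags itself as imploded and destroys itself.
; A delay started on BeginPlay acts as a fallback, spawning the same actor and destroying the arrow if nothing has been hit.
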(event `self.ReceiveBeginPlay`
  ;[0 1 0.8359] If didnt't hit anything, automatically implode
  (`KismetSystemLibrary.Delay` 3.0)
  (if (not (`self.Imploded`))
    (`|SpawnActorFromClass` "/Game/Blueprints/BP_ImplodeAndExplode.BP_ImplodeAndExplode_C" (`self.GetTransform`) "AlwaysSpawn" "OverrideRootScale" null null)
    (`self.K2_DestroyActor`)))

(event `self.Custom Hit`
  (params (`Other Actor` :type "Actor Object Reference") (`Other Comp` :type "PrimitiveComponent Object Reference") (Hit :type "HitResult Structure"))
  (`GameplayStatics.SpawnEmitterAtLocation` "/Game/FXVarietyPack/Particles/P_ky_lightning3.P_ky_lightning3" (`.ImpactPoint` (`GameplayStatics.BreakHitResult` Hit)) (struct) (5.0 5.0 5.0))
  (`|SpawnActorFromClass` "/Game/Blueprints/BP_ImplodeAndExplode.BP_ImplodeAndExplode_C" (`self.GetTransform`) "AlwaysSpawn" "OverrideRootScale" null null)
  (set `self.Imploded` true)
  (`self.K2_DestroyActor`))

(fn `UserConstructionScript`
  (`parent.UserConstructionScript`))