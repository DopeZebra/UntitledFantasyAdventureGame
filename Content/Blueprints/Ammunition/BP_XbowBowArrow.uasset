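; BP_XbowBowArrow is a crossbow arrow projectile that explodes on impact and damages the boss.
; It extends the parent's CustomHit event, spawning a large explosion emitter at the impact point.
; If the hit actor is a BP_BossU, it calls DamageBoss and destroys itself; on other hits this graph stops without destroying the arrow.
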(event `self.Custom Hit`
  (params (`Other Actor` :type "Actor Object Reference") (`Other Comp` :type "PrimitiveComponent Object Reference") (Hit :type "HitResult Structure"))
  (bind (_bblockinghit _binitialoverlap _time _distance _location _impactpoint _normal _impactnormal _physmat _hitactor) (`GameplayStatics.BreakHitResult` Hit))
  (`parent.Custom Hit` `Other Actor` `Other Comp` Hit)
  (`GameplayStatics.SpawnEmitterAtLocation` "/Game/FXVarietyPack/Particles/P_ky_explosion.P_ky_explosion" _impactpoint (struct) (10.0 10.0 10.0))
  (bind _asbp_boss_u (cast `/Game/Blueprints/Characters/Boss/BP_BossU` _hitactor))
  (`/Game/Blueprints/Characters/Boss/BP_BossU.DamageBoss` _asbp_boss_u)
  (`self.K2_DestroyActor`))

(fn `UserConstructionScript`
  (`parent.UserConstructionScript`))