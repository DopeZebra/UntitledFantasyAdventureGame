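; BP_InfiniteArrow_U is an arrow ammunition Blueprint that handles its impact through a CustomHit event.
; The first hit spawns a small particle burst at the impact point.
; Targets implementing DamageInterface_U receive TakeDamageMessage with the NormalArrowDamage value read from the instigating ALS_AnimMan_CharacterBP.
; The arrow then destroys itself, except when a damageable target is hit and that instigator cast fails.
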(event `self.Custom Hit`
  (params (`Other Actor` :type "Actor Object Reference") (`Other Comp` :type "PrimitiveComponent Object Reference") (Hit :type "HitResult Structure"))
  (bind _returnvalue (`self.GetInstigator`))
  (`/Engine/EditorBlueprintResources/StandardMacros.DoOnce` false
    (:`Completed`
      (`GameplayStatics.SpawnEmitterAtLocation` "/Game/FXVarietyPack/Particles/P_ky_hit1.P_ky_hit1" (`.ImpactPoint` (`GameplayStatics.BreakHitResult` Hit)) (struct) (0.2 0.2 0.2))
      (if (`KismetSystemLibrary.DoesImplementInterface` `Other Actor` "/Game/Blueprints/Interface/DamageInterface_U.DamageInterface_U_C")
        (bind _asals_anim_man_character_bp (cast `/Game/AdvancedLocomotionV4/Blueprints/CharacterLogic/Blueprints/ALS_AnimMan_CharacterBP` _returnvalue))
        (message `/Game/Blueprints/Interface/DamageInterface_U.TakeDamage` `Other Actor` `Other Actor` (`/Game/AdvancedLocomotionV4/Blueprints/CharacterLogic/Blueprints/ALS_AnimMan_CharacterBP.Normal Arrow Damage` _asals_anim_man_character_bp) _returnvalue))
      (`self.K2_DestroyActor`))))

(fn `UserConstructionScript`
  (`parent.UserConstructionScript`))