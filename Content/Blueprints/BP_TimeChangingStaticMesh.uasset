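; Actor whose static mesh switches between a past and a present version for a time-travel mechanic.
; The construction script picks the mesh from its Time variable, which Tick then copies from BP_GroupProjectGameState every frame.
; GotoPast, GotoPresent and SwapTime events change the mesh and also write the new time back to the game state, so the actor can drive the shared time.
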(event `self.ReceiveBeginPlay`
  (bind _asbp_group_project_game_state (cast `/Game/Blueprints/GameFiles/BP_GroupProjectGameState` (`GameplayStatics.GetGameState`)))
  (set `self.GS` _asbp_group_project_game_state))

(event `self.ReceiveTick`
  (params (DeltaSeconds :type "Float (single-precision)"))
  (set `self.Time` (`/Game/Blueprints/GameFiles/BP_GroupProjectGameState.Time` (`self.GS`))))

(event `/Game/Blueprints/Interface/TimeChange.GoToPresent`
  (`self.GoTo` "NewEnumerator1"))

(event `/Game/Blueprints/Interface/TimeChange.SwapTime`
  (`self.Swap`))

(event `/Game/Blueprints/Interface/TimeChange.GoToPast`
  (`self.GoTo` "NewEnumerator0"))

(fn `GoTo`
  (params (Time :type "/Game/Blueprints/Data/ENUM_Time Enum" :default "NewEnumerator0"))
  (bind _staticmesh (`self.StaticMesh`))
  (switch `/Game/Blueprints/Data/ENUM_Time` Time
    (:`NewEnumerator0`
      (`StaticMeshComponent.SetStaticMesh` _staticmesh (`self.PastMesh`))
      (set `/Game/Blueprints/GameFiles/BP_GroupProjectGameState.Time` "NewEnumerator0" (`self.GS`)))
    (:`NewEnumerator1`
      (`StaticMeshComponent.SetStaticMesh` _staticmesh (`self.PresentMesh`))
      (set `/Game/Blueprints/GameFiles/BP_GroupProjectGameState.Time` "NewEnumerator1" (`self.GS`)))))

(fn `Swap`
  (switch `/Game/Blueprints/Data/ENUM_Time` (`self.Time`)
    (:`NewEnumerator0`
      (`self.GoTo` "NewEnumerator1")
      (set `/Game/Blueprints/GameFiles/BP_GroupProjectGameState.Time` "NewEnumerator1" (`self.GS`)))
    (:`NewEnumerator1`
      (`self.GoTo` "NewEnumerator0")
      (set `/Game/Blueprints/GameFiles/BP_GroupProjectGameState.Time` "NewEnumerator0" (`self.GS`)))))

(fn `UserConstructionScript`
  (bind _staticmesh (`self.StaticMesh`))
  ;[0.4062 1 0] Set Up mesh according to past or present
  (switch `/Game/Blueprints/Data/ENUM_Time` (`self.Time`)
    (:`NewEnumerator0`
      (`StaticMeshComponent.SetStaticMesh` _staticmesh (`self.PastMesh`)))
    (:`NewEnumerator1`
      (`StaticMeshComponent.SetStaticMesh` _staticmesh (`self.PresentMesh`)))))