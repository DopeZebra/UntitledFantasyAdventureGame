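; Mountable crossbow pawn that the player takes over to aim and fire a single arrow before returning to their character.
; Interact slides the character to the stand point, blends the camera and possesses the crossbow; look inputs rotate its mesh within narrow clamped pitch and yaw.
; Shooting spawns the arrow, tells the game state to switch everything to the present, then shares LeaveXbow's path back to the character.
; Unpossessing resets crossbow and character rotations.
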(event `InputAxis|LookLeft/Right`
  (params (AxisValue :type "Float (single-precision)"))
  (bind (_relativerotation_roll _relativerotation_pitch _relativerotation_yaw) (`KismetMathLibrary.BreakRotator` (`SceneComponent.RelativeRotation` (`self.StaticMesh`))))
  (bind (_returnvalue_roll _returnvalue_pitch _returnvalue_yaw) (`KismetMathLibrary.BreakRotator` (`KismetMathLibrary.MakeRotator` _relativerotation_roll _relativerotation_pitch (+ _relativerotation_yaw (* AxisValue 0.5)))))
  ;[0 0.4844 1] Rotating the Xbow
  (`SceneComponent.K2_SetRelativeRotation` (`self.StaticMesh`) (`KismetMathLibrary.MakeRotator` _returnvalue_roll _returnvalue_pitch (`KismetMathLibrary.ClampAngle` _returnvalue_yaw -5.0 5.0)) false false))

(event `self.ReceiveBeginPlay`
  (bind _asals_anim_man_character_bp (cast `/Game/AdvancedLocomotionV4/Blueprints/CharacterLogic/Blueprints/ALS_AnimMan_CharacterBP` (`GameplayStatics.GetPlayerCharacter` 0)))
  (set `self.Player` _asals_anim_man_character_bp))

(event `InputAxis|LookUp/Down`
  (params (AxisValue :type "Float (single-precision)"))
  (bind (_relativerotation_roll _relativerotation_pitch _relativerotation_yaw) (`KismetMathLibrary.BreakRotator` (`SceneComponent.RelativeRotation` (`self.StaticMesh`))))
  (bind (_returnvalue_roll _returnvalue_pitch _returnvalue_yaw) (`KismetMathLibrary.BreakRotator` (`KismetMathLibrary.MakeRotator` _relativerotation_roll (+ _relativerotation_pitch (* AxisValue 0.5)) _relativerotation_yaw)))
  ;[0 0.4844 1] Rotating the Xbow
  (`SceneComponent.K2_SetRelativeRotation` (`self.StaticMesh`) (`KismetMathLibrary.MakeRotator` _returnvalue_roll (`KismetMathLibrary.ClampAngle` _returnvalue_pitch -10.0 10.0) _returnvalue_yaw) false false))

(event `/Game/Blueprints/Interface/ObjectInterface.Interact`
  (bind _player_stay_location (`self.Player Stay Location`))
  (bind (_returnvalue_roll _returnvalue_pitch _returnvalue_yaw) (`KismetMathLibrary.BreakRotator` (`SceneComponent.K2_GetComponentRotation` (`self.DefaultSceneRoot`))))
  (bind (_relativerotation_roll _relativerotation_pitch _relativerotation_yaw) (`KismetMathLibrary.BreakRotator` (`SceneComponent.RelativeRotation` _player_stay_location)))
  ;[0 0.9766 1] Possess the XBow
  (`KismetSystemLibrary.MoveComponentTo` (`Actor.RootComponent` (`self.Player`)) (`SceneComponent.K2_GetComponentLocation` _player_stay_location) (`KismetMathLibrary.MakeRotator` 0.0 0.0 (+ _relativerotation_yaw _returnvalue_yaw)) true true 0.2)
  (`PlayerController.SetViewTargetWithBlend` (`GameplayStatics.GetPlayerController` 0) self 1.0 "VTBlend_Linear" 0.0 false)
  (`KismetSystemLibrary.Delay` 1.0)
  (`Controller.Possess` (`GameplayStatics.GetPlayerController` 0) self)
  (`self.DisableInput` (`self.Player`) null))

(event `InputAction|Shoot`
  (params (Key :type "Key Structure"))
  ;[1 0.09375 0] Shoot Projectile and give control back to player
  (:`Pressed`
    (`/Engine/EditorBlueprintResources/StandardMacros.DoOnce` false :!label _label
      (:`Completed`
        (`self.ShootProjectile`)
        (`PlayerController.SetViewTargetWithBlend` (`GameplayStatics.GetPlayerController` 0) (`self.Player`) 2.0 "VTBlend_Linear" 0.0 true :!label _label_2)
        (`Controller.Possess` (`GameplayStatics.GetPlayerController` 0) (`self.Player`))
        (`self.EnableInput` (`self.Player`) null)
        (goto _label :!via `Reset`)))))

(event `LeaveXbow`
  ;[1 0.09375 0] Shoot Projectile and give control back to player
  (`Controller.UnPossess` (`GameplayStatics.GetPlayerController` 0))
  (goto _label_2))

(event `ShootProjectile`
  ;[1 0.09375 0] Shoot Projectile and give control back to player
  (`|SpawnActorFromClass` "/Game/Blueprints/Ammunition/BP_XbowBowArrow.BP_XbowBowArrow_C" (`SceneComponent.K2_GetComponentToWorld` (`self.Arrow`)) "Undefined" "OverrideRootScale" null (`self.Player`) null)
  (bind _asbp_group_project_game_state (cast `/Game/Blueprints/GameFiles/BP_GroupProjectGameState` (`GameplayStatics.GetGameState`)))
  (`/Game/Blueprints/GameFiles/BP_GroupProjectGameState.ChangeEverythingToPresent` _asbp_group_project_game_state))

(event `self.ReceiveUnpossessed`
  (params (OldController :type "Controller Object Reference"))
  ;[1 0.1875 0] Reset player and XBow Rotation
  (`SceneComponent.K2_SetRelativeRotation` :`self` (`self.StaticMesh`))
  (`SceneComponent.K2_SetWorldRotation` (`Actor.RootComponent` (`self.Player`)) (`SceneComponent.K2_GetComponentRotation` (`self.Player Stay Location`)) false false))

(fn `UserConstructionScript`)