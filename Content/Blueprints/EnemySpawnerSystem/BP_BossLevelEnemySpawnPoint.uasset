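; Boss-level spawn point actor that spawns a wave of enemies for the boss fight.
; SpawnEnemy reads the wave entry for the Boss's current wave, spawns that count of its enemy type, then reports the spawned total back to the Boss.
; The Spawn Actors macro maps the type to Undin, OxBaren or Agnar classes, placing each at a random point inside the Box and tagging it "Boss".
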(event `self.ReceiveBeginPlay`)

(fn `SpawnEnemy`
  (bind (_returnvalue_location _returnvalue_rotation) (`KismetMathLibrary.BreakTransform` (`self.GetTransform`)))
  (bind _returnvalue (`KismetMathLibrary.RandomPointInBoundingBox` (`SceneComponent.K2_GetComponentLocation` (`self.DefaultSceneRoot`)) (`BoxComponent.GetScaledBoxExtent` (`self.Box`))))
  (bind (_enemytype _numberofenemiestospawn) (break `/Game/Blueprints/EnemySpawnerSystem/EnemySpawnInfo` (`|GetArrayItem` (`self.WaveSpawner`) (`/Game/Blueprints/Characters/Boss/BP_BossU.CurrentWave` (`self.Boss`)))))
  (set `self.TempNumberOfEnemiesSpawned` 0)
  (for _ (range _numberofenemiestospawn)
    (switch `/Game/Blueprints/Data/ENUM_EnemyType` _enemytype
      (:`NewEnumerator0`
        (`|SpawnActorFromClass` "/Game/Blueprints/Characters/Enemy01/BP_Undin.BP_Undin_C" (`KismetMathLibrary.MakeTransform` _returnvalue _returnvalue_rotation) "AlwaysSpawn" "OverrideRootScale" null null "Boss" null))
      (:`NewEnumerator1`
        (`|SpawnActorFromClass` "/Game/Blueprints/Characters/Enemy02/BP_OxBaren.BP_OxBaren_C" (`KismetMathLibrary.MakeTransform` _returnvalue) "AdjustIfPossibleButAlwaysSpawn" "OverrideRootScale" null null "Boss" null))
      (:`NewEnumerator2`
        (`|SpawnActorFromClass` "/Game/Blueprints/Characters/Enemy03/BP_TestE03.BP_TestE03_C" (`KismetMathLibrary.MakeTransform` _returnvalue _returnvalue_rotation) "Undefined" "OverrideRootScale" null null "Boss" null)))
    (`/Engine/EditorBlueprintResources/StandardMacros.IncrementInt` (`self.TempNumberOfEnemiesSpawned`)))
  (`/Game/Blueprints/Characters/Boss/BP_BossU.CalculateNumberofSpawnedEnemies` (`self.Boss`) (`self.TempNumberOfEnemiesSpawned`)))

(fn `UserConstructionScript`)