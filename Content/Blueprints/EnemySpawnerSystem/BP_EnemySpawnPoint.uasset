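; BP_EnemySpawnPoint is a placed spawn point that spawns enemies for the current wave at its own location and rotation.
; SpawnEnemy reads its WaveSpawner entry at the SpawnManager's current wave number to get the enemy count and type, mapping the type to one of three test enemy Blueprints.
; It then passes the number spawned to the SpawnManager's CalculateNumberofSpawnedEnemies.
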(fn `SpawnEnemy`
  (bind (_returnvalue_location _returnvalue_rotation) (`KismetMathLibrary.BreakTransform` (`self.GetTransform`)))
  (bind (_enemytype _numberofenemiestospawn) (break `/Game/Blueprints/EnemySpawnerSystem/EnemySpawnInfo` (`|GetArrayItem` (`self.WaveSpawner`) (`/Game/Blueprints/EnemySpawnerSystem/BP_SpawnManager.CurrentWaveNumber` (`self.SpawnManager`)))))
  (set `self.TempNumberOfEnemiesSpawned` 0)
  (for _ (range (+ _numberofenemiestospawn 1))
    (`|SpawnActorFromClass` (select `/Game/Blueprints/Data/ENUM_EnemyType` _enemytype :`NewEnumerator0` "/Game/Blueprints/Characters/Enemy01/BP_TestE01.BP_TestE01_C" :`NewEnumerator1` "/Game/Blueprints/Characters/Enemy02/BP_TestE02.BP_TestE02_C" :`NewEnumerator2` "/Game/Blueprints/Characters/Enemy03/BP_TestE03.BP_TestE03_C" :!type "Actor Class Reference") (`KismetMathLibrary.MakeTransform` _returnvalue_location _returnvalue_rotation) "AdjustIfPossibleButAlwaysSpawn" "OverrideRootScale" self null)
    (`/Engine/EditorBlueprintResources/StandardMacros.IncrementInt` (`self.TempNumberOfEnemiesSpawned`)))
  (`/Game/Blueprints/EnemySpawnerSystem/BP_SpawnManager.CalculateNumberofSpawnedEnemies` (`self.SpawnManager`) (`self.TempNumberOfEnemiesSpawned`)))

(fn `UserConstructionScript`)