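; Actor that pulls nearby physics objects inward for two seconds, then explodes and destroys itself.
; On BeginPlay it gathers WorldDynamic components in a sphere once, enables physics on them and repeatedly adds velocity toward its center on a looping timer.
; It then fires a radial force impulse with an explosion emitter.
; Tick-triggered timelines shrink and expand a sphere as the shockwave, destroying the actor when expansion finishes.
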(event `self.ReceiveBeginPlay`
  (`self.Implode`)
  (bind _returnvalue (`KismetSystemLibrary.K2_SetTimerDelegate` (delegate `Implode`) 0.1 true))
  (bind _output_get (set `self.Implde Timer` _returnvalue))
  (`KismetSystemLibrary.Delay` 2.0)
  (`KismetSystemLibrary.K2_ClearAndInvalidateTimerHandle` _output_get)
  (`self.Explode`))

(event `Implode`
  (bind _returnvalue (`self.K2_GetActorLocation`))
  (`|ExecutionSequence`
    (:`then_0`
      (`/Engine/EditorBlueprintResources/StandardMacros.DoOnce` false
        (:`Completed`
          (`KismetSystemLibrary.DrawDebugSphere` _returnvalue 1000.0 12 (struct :`R` 0.112093 :`G` 0.00152 :`B` 1.0 :`A` 1.0) 2.0 1.0)
          (bind _outcomponents (`KismetSystemLibrary.SphereOverlapComponents` _returnvalue 1000.0 (`|MakeArray` "ObjectTypeQuery2" :!type "EObjectTypeQuery Enum")))
          (bind _output_get (set `self.Objects` _outcomponents))
          (`KismetSystemLibrary.PrintString` (`KismetStringLibrary.Conv_IntToString` (`KismetArrayLibrary.Array_Length` _output_get))))))
    (:`then_1`
      (set `self.Imploding` true))
    (:`then_2`
      (if (> (`KismetArrayLibrary.Array_Length` (`self.Objects`)) 0)
        (for _array_element (`self.Objects`)
          (`PrimitiveComponent.SetSimulatePhysics` _array_element true)
          (`PrimitiveComponent.SetMassOverrideInKg` _array_element "None" 1.0 true))
        (for _array_element_2 (`self.Objects`)
          (`PrimitiveComponent.SetPhysicsLinearVelocity` _array_element_2 (* (`KismetMathLibrary.GetForwardVector` (`KismetMathLibrary.FindLookAtRotation` (`SceneComponent.K2_GetComponentLocation` _array_element_2) (`self.K2_GetActorLocation`))) 700.0) true "None"))))))

(event `self.ReceiveTick`
  (params (DeltaSeconds :type "Float (single-precision)"))
  (`|ExecutionSequence`
    (:`then_0`
      (if (`self.Imploding`)
        (`/Engine/EditorBlueprintResources/StandardMacros.DoOnce` false
          (:`Completed`
            (bind (_direction _lerp) (`Timeline|ReduceImplosionShockWave` :!via `PlayFromStart`)
              (:`Update`
                (`SceneComponent.SetRelativeScale3D` (`self.Sphere`) (`KismetMathLibrary.VLerp` (15.0 15.0 15.0) (0.0 0.0 0.0) _lerp))))))))
    (:`then_1`
      (if (`self.Exploding`)
        (`/Engine/EditorBlueprintResources/StandardMacros.DoOnce` false
          (:`Completed`
            (bind (_direction_2 _lerp_2) (`Timeline|Timeline_0` :!via `PlayFromStart`)
              (:`Update`
                (`SceneComponent.SetRelativeScale3D` (`self.Sphere`) (`KismetMathLibrary.VLerp` (0.0 0.0 0.0) (50.0 50.0 500.0) _lerp_2)))
              (:`Finished`
                (`self.K2_DestroyActor`)))))))))

(event `Explode`
  (bind (_returnvalue_location _returnvalue_rotation) (`KismetMathLibrary.BreakTransform` (`self.GetTransform`)))
  (set `self.Exploding` true)
  (set `self.Imploding` false)
  (`GameplayStatics.SpawnEmitterAtLocation` "/Game/StarterContent/Particles/P_Explosion.P_Explosion" _returnvalue_location _returnvalue_rotation (5.0 5.0 5.0))
  (`KismetSystemLibrary.PrintString` "Explode")
  (`RadialForceComponent.FireImpulse` (`self.RadialForce`)))

(fn `UserConstructionScript`)