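; Actor that switches the level's look between Past and Present by toggling two post process components, PastPP and PresentPP.
; Swap flips the era and sets the "Time" audio state, while GoTo forces a given era without changing audio.
; Both write the era to BP_GroupProjectGameState, which Tick copies back into the local Time variable.
; The construction script applies the matching post process for the initial Time.
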(event `self.ReceiveBeginPlay`
  (bind _asbp_group_project_game_state (cast `/Game/Blueprints/GameFiles/BP_GroupProjectGameState` (`GameplayStatics.GetGameState`)))
  (set `self.GS` _asbp_group_project_game_state))

(event `self.ReceiveTick`
  (params (DeltaSeconds :type "Float (single-precision)"))
  (set `self.Time` (`/Game/Blueprints/GameFiles/BP_GroupProjectGameState.Time` (`self.GS`))))

(event `/Game/Blueprints/Interface/TimeChange.GoToPresent`
  (`self.GoTo` "NewEnumerator1"))

(event `/Game/Blueprints/Interface/TimeChange.SwapTime`
  (`self.Swap`))

(event `/Game/Blueprints/Interface/TimeChange.GoToPast`
  (`self.GoTo` "NewEnumerator0"))

(fn `GoTo`
  (params (Time :type "/Game/Blueprints/Data/ENUM_Time Enum" :default "NewEnumerator0"))
  (switch `/Game/Blueprints/Data/ENUM_Time` Time
    (:`NewEnumerator0`
      (set `PostProcessVolume.bEnabled` true (`self.PastPP`))
      (set `PostProcessVolume.bEnabled` false (`self.PresentPP`))
      (set `/Game/Blueprints/GameFiles/BP_GroupProjectGameState.Time` "NewEnumerator0" (`self.GS`)))
    (:`NewEnumerator1`
      (set `PostProcessVolume.bEnabled` false (`self.PastPP`))
      (set `PostProcessVolume.bEnabled` true (`self.PresentPP`))
      (set `/Game/Blueprints/GameFiles/BP_GroupProjectGameState.Time` "NewEnumerator1" (`self.GS`)))))

(fn `Swap`
  (switch `/Game/Blueprints/Data/ENUM_Time` (`self.Time`)
    (:`NewEnumerator0`
      (set `PostProcessVolume.bEnabled` false (`self.PastPP`))
      (set `PostProcessVolume.bEnabled` true (`self.PresentPP`))
      (set `/Game/Blueprints/GameFiles/BP_GroupProjectGameState.Time` "NewEnumerator1" (`self.GS`))
      ;[0.2678 0.9022 1] Audio
      (`AkGameplayStatics.SetState` "Time" "Present"))
    (:`NewEnumerator1`
      (set `PostProcessVolume.bEnabled` true (`self.PastPP`))
      (set `PostProcessVolume.bEnabled` false (`self.PresentPP`))
      (set `/Game/Blueprints/GameFiles/BP_GroupProjectGameState.Time` "NewEnumerator0" (`self.GS`))
      (`AkGameplayStatics.SetState` "Time" "Past"))))

(fn `UserConstructionScript`
  (switch `/Game/Blueprints/Data/ENUM_Time` (`self.Time`)
    (:`NewEnumerator0`
      (set `PostProcessVolume.bEnabled` true (`self.PastPP`))
      (set `PostProcessVolume.bEnabled` false (`self.PresentPP`)))
    (:`NewEnumerator1`
      (set `PostProcessVolume.bEnabled` false (`self.PastPP`))
      (set `PostProcessVolume.bEnabled` true (`self.PresentPP`)))))