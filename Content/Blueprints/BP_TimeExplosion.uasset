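; Time-slow explosion actor that drags down the time dilation of nearby actors for about five seconds, sparing the player character.
; Tick and a looping timer both call SlowTIme, whose delayed multi-sphere trace records hit actors and slows them.
; EndTask restores normal dilation on the recorded actors, then destroys this actor from inside its second loop.
; Older overlap-based variants remain disconnected, including the only use of the gathered BP_Undin list.
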(event `EndTask`
  (for _array_element (`self.ComponentHitList`)
    (`KismetSystemLibrary.PrintString` (`KismetSystemLibrary.GetDisplayName` _array_element))
    (set `Actor.CustomTimeDilation` 1.0 _array_element))
  (`KismetSystemLibrary.Delay` 0.1)
  (for _array_element_2 (`self.ComponentHitList`)
    (set `Actor.CustomTimeDilation` 1.0 _array_element_2)
    (`self.K2_DestroyActor`)))

(event `self.ReceiveTick`
  (params (DeltaSeconds :type "Float (single-precision)"))
  (`self.SlowTIme`))

(event `self.ReceiveBeginPlay`
  (bind _outactors (`GameplayStatics.GetAllActorsOfClass` "/Game/Blueprints/Characters/Enemy01/BP_Undin.BP_Undin_C"))
  (set `self.AllUndin` _outactors)
  (bind _asals_anim_man_character_bp (cast `/Game/AdvancedLocomotionV4/Blueprints/CharacterLogic/Blueprints/ALS_AnimMan_CharacterBP` (`GameplayStatics.GetPlayerPawn` 0)))
  (bind _output_get (set `self.CharRefrence` _asals_anim_man_character_bp))
  (bind _outactors_2 (`GameplayStatics.GetAllActorsOfClass` "/Game/AdvancedLocomotionV4/Blueprints/CameraSystem/Blueprints/ALS_PlayerCameraManager.ALS_PlayerCameraManager_C"))
  (set `self.CameraRefrence` (`|GetArrayItem` _outactors_2))
  (`|ExecutionSequence`
    (:`then_0`
      (`KismetSystemLibrary.Delay` 5.0)
      (set `Actor.CustomTimeDilation` 1.0 (`self.CharRefrence`))
      (`self.EndTask`))
    (:`then_1`
      (`KismetSystemLibrary.K2_SetTimerDelegate` (delegate `SlowTIme`) 0.1 true)
      (set `Actor.CustomTimeDilation` 1.0 _output_get))))

(event `SlowTIme`
  (bind _returnvalue (`self.K2_GetActorLocation`))
  (bind _componenttonotaffectedbyarrow (`self.ComponentToNotAffectedByArrow`))
  (`|ExecutionSequence`
    (:`then_0`
      (`/Engine/EditorBlueprintResources/StandardMacros.DoOnce` false))
    (:`then_1`
      (`KismetSystemLibrary.Delay` 0.2)
      (`KismetArrayLibrary.Array_Add` _componenttonotaffectedbyarrow (`self.CharRefrence`))
      (bind _outhits (`KismetSystemLibrary.SphereTraceMulti` _returnvalue _returnvalue 1000.0 "TraceTypeQuery2" true _componenttonotaffectedbyarrow "ForOneFrame"))
      (for _array_element _outhits
        (bind (_bblockinghit _binitialoverlap _time _distance _location _impactpoint _normal _impactnormal _physmat _hitactor) (`GameplayStatics.BreakHitResult` _array_element))
        (`KismetArrayLibrary.Array_Add` (`self.ComponentHitList`) _hitactor)
        (set `Actor.CustomTimeDilation` 0.1 _hitactor)))))

(fn `UserConstructionScript`)