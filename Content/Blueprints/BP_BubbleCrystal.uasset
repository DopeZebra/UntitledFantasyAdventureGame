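; BP_BubbleCrystal is a crystal actor that breaks loose when damaged and explodes on impact to grow a bubble.
; Damage turns on mesh physics and disables actor collision for a short delay before restoring it.
; The first mesh hit, guarded by DoOnce, spawns an explosion, calls PlayGrowBubble on the Bubble reference and destroys the crystal.
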(event `/Game/Blueprints/Interface/DamageInterface_U.TakeDamage`
  (params (DamagedActor :type "Actor Object Reference") (DamageToApply :type "Float (single-precision)") (DamageCauser :type "Actor Object Reference"))
  (`self.SetActorEnableCollision` false)
  (`PrimitiveComponent.SetSimulatePhysics` (`self.StaticMesh`) true)
  (`KismetSystemLibrary.Delay` 0.5)
  (`self.SetActorEnableCollision` true))

(event `self.StaticMesh.OnComponentHit`
  (params (HitComponent :type "PrimitiveComponent Object Reference") (OtherActor :type "Actor Object Reference") (OtherComp :type "PrimitiveComponent Object Reference") (NormalImpulse :type "Vector Structure") (Hit :type "HitResult Structure (by ref)"))
  (bind (_returnvalue_location _returnvalue_rotation) (`KismetMathLibrary.BreakTransform` (`self.GetTransform`)))
  (`/Engine/EditorBlueprintResources/StandardMacros.DoOnce` false
    (:`Completed`
      (`GameplayStatics.SpawnEmitterAtLocation` "/Game/StarterContent/Particles/P_Explosion.P_Explosion" _returnvalue_location _returnvalue_rotation)
      (`/Game/Blueprints/BP_Bubble.PlayGrowBubble` (`self.Bubble`))
      (`self.K2_DestroyActor`))))

(fn `UserConstructionScript`)