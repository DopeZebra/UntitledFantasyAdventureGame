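; BP_Unidn is an enemy character that is tracked by a spawn manager and linked to an AI_UndinController.
; On BeginPlay it takes the manager from its owning spawn point, tags itself with its controlling side, reads its controller's ID after a short delay and sets walking movement.
; When destroyed, it decrements and prints the manager's enemy count.
; Tick calls PlayFootsteps while moving, but that event is empty.
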(event `self.ReceiveBeginPlay`
  (`|ExecutionSequence`
    (:`then_0`
      (bind _asbp_enemy_spawn_point (cast `/Game/Blueprints/EnemySpawnerSystem/BP_EnemySpawnPoint` (`self.GetOwner`)))
      (set `self.SpawnManager` (`/Game/Blueprints/EnemySpawnerSystem/BP_EnemySpawnPoint.SpawnManager` _asbp_enemy_spawn_point)))
    (:`then_1`
      ;[0 0.1094 1] Tag to set who is controlling this enemy (Usually handled by the spawner)
      (set `self.Tags` (`|MakeArray` (`self.Tag`))))
    (:`then_2`
      (`KismetSystemLibrary.Delay` 0.5)
      (bind _asai_undin_controller (cast `/Game/Blueprints/Characters/Enemy01/UndinAI/AI_UndinController` (`AIBlueprintHelperLibrary.GetAIController` self)))
      (set `self.IdNumber` (`/Game/Blueprints/Characters/Enemy01/UndinAI/AI_UndinController.IDNumber` _asai_undin_controller)))
    (:`then_3`
      (`CharacterMovementComponent.SetMovementMode` (`self.CharacterMovement`) "MOVE_Walking" 0))))

(event `self.ReceiveTick`
  (params (DeltaSeconds :type "Float (single-precision)"))
  (if (> (`KismetMathLibrary.VSize` (`MovementComponent.Velocity` (`self.CharacterMovement`))) 0.0)
    (`self.PlayFootsteps`)))

(event `PlayFootsteps`)

(event `self.ReceiveDestroyed`
  (bind _spawnmanager (`self.SpawnManager`))
  (`/Engine/EditorBlueprintResources/StandardMacros.IsValid` _spawnmanager
    (:`Is Valid`
      (bind _output_get (set `/Game/Blueprints/EnemySpawnerSystem/BP_SpawnManager.NumberOfEnemies` (- (`/Game/Blueprints/EnemySpawnerSystem/BP_SpawnManager.NumberOfEnemies` _spawnmanager) 1) _spawnmanager))
      (`KismetSystemLibrary.PrintString` (`KismetStringLibrary.Concat_StrStr` "Number of enemies left" (`KismetStringLibrary.Conv_IntToString` _output_get))))))

(fn `UserConstructionScript`)