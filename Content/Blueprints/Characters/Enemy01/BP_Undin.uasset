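; Undin enemy character: a melee attacker that damages the player and reports its removal to a spawn manager.
; Hand collisions are active only while attacking, sending damage on player hits with a one-second per-hand reset.
; Incoming damage lowers health until death triggers a ragdoll and timeline-driven dissolve of two dynamic materials, then destruction.
; The spawn manager comes from the owning spawn point, and its enemy count decrements on destruction.
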(event `self.ReceiveBeginPlay`
  (`|ExecutionSequence`
    (:`then_0`
      (bind _asbp_enemy_spawn_point (cast `/Game/Blueprints/EnemySpawnerSystem/BP_EnemySpawnPoint` (`self.GetOwner`)))
      (set `self.SpawnManager` (`/Game/Blueprints/EnemySpawnerSystem/BP_EnemySpawnPoint.SpawnManager` _asbp_enemy_spawn_point)))
    (:`then_1`
      ;[0 0.1094 1] Tag to set who is controlling this enemy (Usually handled by the spawner)
      (set `self.Tags` (`|MakeArray` (`self.Tag`))))
    (:`then_2`
      (`KismetSystemLibrary.Delay` 0.5)
      (bind _asai_undin_controller (cast `/Game/Blueprints/Characters/Enemy01/UndinAI/AI_UndinController` (`AIBlueprintHelperLibrary.GetAIController` self)))
      (set `self.IdNumber` (`/Game/Blueprints/Characters/Enemy01/UndinAI/AI_UndinController.IDNumber` _asai_undin_controller)))
    (:`then_3`
      (`CharacterMovementComponent.SetMovementMode` (`self.CharacterMovement`) "MOVE_NavWalking" 0))
    (:`then_4`
      (set `self.Current Health` (`self. Max Health`)))
    (:`then_5`
      (bind _returnvalue (`PrimitiveComponent.CreateDynamicMaterialInstance` (`self.Mesh`) 0 "/Game/Material/M_UP01.M_UP01" "None"))
      (`KismetArrayLibrary.Array_Add` (`self.Materials`) _returnvalue)
      (bind _returnvalue_2 (`PrimitiveComponent.CreateDynamicMaterialInstance` (`self.Mesh`) 1 "/Game/Material/M_UP01.M_UP01" "None"))
      (`KismetArrayLibrary.Array_Add` (`self.Materials`) _returnvalue_2))))

(event `self.ReceiveTick`
  (params (DeltaSeconds :type "Float (single-precision)"))
  (`|ExecutionSequence`
    (:`then_0`
      (if (> (`KismetMathLibrary.VSize` (`MovementComponent.Velocity` (`self.CharacterMovement`))) 0.0)
        (`self.PlayFootsteps`)))
    (:`then_1`
      (if (`self.isAttacking`)
        (`PrimitiveComponent.SetCollisionEnabled` (`self.Left Hand Collision`) "QueryAndPhysics")
        (`PrimitiveComponent.SetCollisionEnabled` (`self.Right Hand COllision`) "QueryAndPhysics")
        (else
          (`PrimitiveComponent.SetCollisionEnabled` (`self.Left Hand Collision`) "NoCollision")
          (`PrimitiveComponent.SetCollisionEnabled` (`self.Right Hand COllision`) "NoCollision"))))))

(event `PlayFootsteps`)

(event `self.Right Hand COllision.OnComponentHit`
  (params (HitComponent :type "PrimitiveComponent Object Reference") (OtherActor :type "Actor Object Reference") (OtherComp :type "PrimitiveComponent Object Reference") (NormalImpulse :type "Vector Structure") (Hit :type "HitResult Structure (by ref)"))
  (`/Engine/EditorBlueprintResources/StandardMacros.DoOnce` false :!label _label
    (:`Completed`
      (if (== OtherActor (`GameplayStatics.GetPlayerPawn` 0))
        (bind _asals_anim_man_character_bp (cast `/Game/AdvancedLocomotionV4/Blueprints/CharacterLogic/Blueprints/ALS_AnimMan_CharacterBP` (`GameplayStatics.GetPlayerPawn` 0)))
        (message `/Game/Blueprints/Interface/DamageInterface_U.TakeDamage` _asals_anim_man_character_bp _asals_anim_man_character_bp (`self.Damage Amount`) self)
        (`KismetSystemLibrary.Delay` 1.0)
        (goto _label :!via `Reset`)))))

(event `self.Left Hand Collision.OnComponentHit`
  (params (HitComponent :type "PrimitiveComponent Object Reference") (OtherActor :type "Actor Object Reference") (OtherComp :type "PrimitiveComponent Object Reference") (NormalImpulse :type "Vector Structure") (Hit :type "HitResult Structure (by ref)"))
  (`/Engine/EditorBlueprintResources/StandardMacros.DoOnce` false :!label _label_2
    (:`Completed`
      (if (== OtherActor (`GameplayStatics.GetPlayerPawn` 0))
        (bind _asals_anim_man_character_bp (cast `/Game/AdvancedLocomotionV4/Blueprints/CharacterLogic/Blueprints/ALS_AnimMan_CharacterBP` (`GameplayStatics.GetPlayerPawn` 0)))
        (message `/Game/Blueprints/Interface/DamageInterface_U.TakeDamage` _asals_anim_man_character_bp _asals_anim_man_character_bp (`self.Damage Amount`) self)
        (`KismetSystemLibrary.Delay` 1.0)
        (goto _label_2 :!via `Reset`)))))

(event `/Game/Blueprints/Interface/DamageInterface_U.TakeDamage`
  (params (DamagedActor :type "Actor Object Reference") (DamageToApply :type "Float (single-precision)") (DamageCauser :type "Actor Object Reference"))
  (`KismetSystemLibrary.PrintString` "Hello")
  (bind _output_get (set `self.Current Health` (`/Game/Blueprints/CustomMacroLibraries/ML_HealthAndDamage.FloorHealthValue` (`/Game/Blueprints/CustomMacroLibraries/ML_HealthAndDamage.ReduceHealth` (`self.Current Health`) DamageToApply))))
  (if (`/Game/Blueprints/CustomMacroLibraries/ML_HealthAndDamage.HealthCheck` _output_get)
    (`self.OnDeath`)
    (else
      (`KismetSystemLibrary.PrintString` (`KismetStringLibrary.Conv_DoubleToString` _output_get) true true (struct :`R` 1.0 :`G` 0.02496 :`A` 1.0)))))

(event `OnDeath`
  ;[0.3594 1 0] On Death
  (`/Engine/EditorBlueprintResources/StandardMacros.DoOnce` false
    (:`Completed`
      (`NavMovementComponent.StopActiveMovement` (`self.CharacterMovement`))
      (`PrimitiveComponent.SetCollisionEnabled` (`self.Mesh`) "QueryAndPhysics")
      (`PrimitiveComponent.SetCollisionResponseToChannel` (`self.CapsuleComponent`) "ECC_GameTraceChannel2" "ECR_Ignore")
      (`SkeletalMeshComponent.SetAllBodiesBelowSimulatePhysics` (`self.Mesh`) (`self.Bone Name`) true true)
      (`|ExecutionSequence`
        (:`then_0`
          (bind (_direction _newtrack_0) (`Timeline|Dissolve` :!via `PlayFromStart`)
            (:`Update`
              (`MaterialInstanceDynamic.SetScalarParameterValue` (`|GetArrayItem` (`self.Materials`)) "Dissolve Amount" _newtrack_0))))
        (:`then_1`
          (bind (_direction_2 _newtrack_0_2) (`Timeline|Timeline_0` :!via `PlayFromStart`)
            (:`Update`
              (`MaterialInstanceDynamic.SetScalarParameterValue` (`|GetArrayItem` (`self.Materials`) 1) "Dissolve Amount" _newtrack_0_2))
            (:`Finished`
              (`self.K2_DestroyActor`))))))))

(event `self.ReceiveDestroyed`
  (bind _spawnmanager (`self.SpawnManager`))
  ;[0.3594 1 0] On Death
  (`/Engine/EditorBlueprintResources/StandardMacros.IsValid` _spawnmanager
    (:`Is Valid`
      (bind _output_get (set `/Game/Blueprints/EnemySpawnerSystem/BP_SpawnManager.NumberOfEnemies` (- (`/Game/Blueprints/EnemySpawnerSystem/BP_SpawnManager.NumberOfEnemies` _spawnmanager) 1) _spawnmanager))
      (`KismetSystemLibrary.PrintString` (`KismetStringLibrary.Concat_StrStr` "Number of enemies left" (`KismetStringLibrary.Conv_IntToString` _output_get))))))

(fn `UserConstructionScript`)