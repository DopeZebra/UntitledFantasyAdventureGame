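; BP_ShockWave is an enemy shockwave actor that expands outward from where it spawns and detects when it hits the player's ALS-based character.
; On BeginPlay a timeline scales the InnerRing component in X and Y while keeping its Z, then destroys the actor when it finishes.
; An overlap on InnerRing is gated by a DoOnce and currently only prints a debug hit message, with no damage applied.
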(event `self.ReceiveBeginPlay`
  (bind (_returnvalue_x _returnvalue_y _returnvalue_z) (`KismetMathLibrary.BreakVector` (`SceneComponent.K2_GetComponentScale` (`self.InnerRing`))))
  (bind (_direction _newtrack_0) (`Timeline|ShockwaveGrow` :!via `PlayFromStart`)
    (:`Update`
      (`SceneComponent.SetRelativeScale3D` (`self.InnerRing`) (`KismetMathLibrary.MakeVector` (* _newtrack_0 0.5) (* 0.5 _newtrack_0) _returnvalue_z)))
    (:`Finished`
      (`self.K2_DestroyActor`))))

(event `self.InnerRing.OnComponentBeginOverlap`
  (params (OverlappedComponent :type "PrimitiveComponent Object Reference") (OtherActor :type "Actor Object Reference") (OtherComp :type "PrimitiveComponent Object Reference") (OtherBodyIndex :type Integer) (bFromSweep :type Boolean) (SweepResult :type "HitResult Structure (by ref)"))
  (cast `/Game/AdvancedLocomotionV4/Blueprints/CharacterLogic/Blueprints/ALS_AnimMan_CharacterBP` OtherActor)
  (`/Engine/EditorBlueprintResources/StandardMacros.DoOnce` false
    (:`Completed`
      (`KismetSystemLibrary.PrintString` "Shockwave Hit"))))

(fn `UserConstructionScript`)