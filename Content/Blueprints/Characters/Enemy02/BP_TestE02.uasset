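; BP_TestE02 is a test enemy that removes itself after a random lifespan and updates the spawn manager's enemy count.
; On BeginPlay it casts its owner to BP_EnemySpawnPoint, caches that point's SpawnManager, then sets the lifespan; a failed cast skips both.
; When destroyed, it decrements the manager's NumberOfEnemies and prints the remaining count.
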(event `self.ReceiveBeginPlay`
  (bind _asbp_enemy_spawn_point (cast `/Game/Blueprints/EnemySpawnerInformation/BP_EnemySpawnPoint` (`self.GetOwner`)))
  (set `self.SpawnManager` (`/Game/Blueprints/EnemySpawnerInformation/BP_EnemySpawnPoint.SpawnManager` _asbp_enemy_spawn_point))
  (`self.SetLifeSpan` (`KismetMathLibrary.RandomFloatInRange` 7.0 10.0)))

(event `self.ReceiveDestroyed`
  (bind _spawnmanager (`self.SpawnManager`))
  (bind _output_get (set `/Game/Blueprints/EnemySpawnerInformation/BP_SpawnManager.NumberOfEnemies` (- (`/Game/Blueprints/EnemySpawnerInformation/BP_SpawnManager.NumberOfEnemies` _spawnmanager) 1) _spawnmanager))
  (`KismetSystemLibrary.PrintString` (`KismetStringLibrary.Concat_StrStr` "Number of enemies left" (`KismetStringLibrary.Conv_IntToString` _output_get))))

(fn `UserConstructionScript`)