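; BP_OxBaren is an enemy actor that reports its removal to a spawn manager and can explode.
; On BeginPlay it caches the SpawnManager from its owning BP_EnemySpawnPoint and sets its actor tags from its Tag variable.
; When destroyed, it decrements that manager's enemy count, if valid, and prints the remainder.
; ExplodeActor spawns an enlarged explosion particle at its location, then destroys the actor.
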(event `self.ReceiveBeginPlay`
  (`|ExecutionSequence`
    (:`then_0`
      (bind _asbp_enemy_spawn_point (cast `/Game/Blueprints/EnemySpawnerSystem/BP_EnemySpawnPoint` (`self.GetOwner`)))
      (set `self.SpawnManager` (`/Game/Blueprints/EnemySpawnerSystem/BP_EnemySpawnPoint.SpawnManager` _asbp_enemy_spawn_point)))
    (:`then_1`
      (set `self.Tags` (`|MakeArray` (`self.Tag`))))))

(event `self.ReceiveTick`
  (params (DeltaSeconds :type "Float (single-precision)")))

(event `self.ReceiveDestroyed`
  (bind _spawnmanager (`self.SpawnManager`))
  (`/Engine/EditorBlueprintResources/StandardMacros.IsValid` _spawnmanager
    (:`Is Valid`
      (bind _output_get (set `/Game/Blueprints/EnemySpawnerSystem/BP_SpawnManager.NumberOfEnemies` (- (`/Game/Blueprints/EnemySpawnerSystem/BP_SpawnManager.NumberOfEnemies` _spawnmanager) 1) _spawnmanager))
      (`KismetSystemLibrary.PrintString` (`KismetStringLibrary.Concat_StrStr` "Number of enemies left" (`KismetStringLibrary.Conv_IntToString` _output_get))))))

(event `ExplodeActor`
  (`GameplayStatics.SpawnEmitterAtLocation` "/Game/StarterContent/Particles/P_Explosion.P_Explosion" (`self.K2_GetActorLocation`) (struct) (5.0 5.0 5.0))
  (`self.K2_DestroyActor`))

(fn `UserConstructionScript`)