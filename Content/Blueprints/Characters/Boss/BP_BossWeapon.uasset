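; BP_BossWeapon is the boss's sword actor, hidden with collision off at start and toggled by SpawnSingleSword and DisappearSword events.
; When Sword01 overlaps the player, it launches them along world Y, sends a damage message and calls the boss's post-hit charge-time event.
; A DoOnce gate limits repeat hits until a non-player overlap or ResetDoOnce resets it.
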(event `self.ReceiveBeginPlay`
  (`self.SetActorHiddenInGame` true)
  (`self.SetActorEnableCollision` false))

(event `SpawnSingleSword`
  (`self.SetActorHiddenInGame` false)
  (`self.SetActorEnableCollision` true))

(event `self.Sword01.OnComponentBeginOverlap`
  (params (OverlappedComponent :type "PrimitiveComponent Object Reference") (OtherActor :type "Actor Object Reference") (OtherComp :type "PrimitiveComponent Object Reference") (OtherBodyIndex :type Integer) (bFromSweep :type Boolean) (SweepResult :type "HitResult Structure (by ref)"))
  (bind _returnvalue (`GameplayStatics.GetPlayerCharacter` 0))
  ;[1 0.1172 0] Hitting the player
  (if (== OtherActor _returnvalue)
    (`/Engine/EditorBlueprintResources/StandardMacros.DoOnce` false :!label _label
      (:`Completed`
        (`Character.LaunchCharacter` _returnvalue (0.0 500.0 0.0) true false)
        (message `/Game/Blueprints/Interface/DamageInterface_U.TakeDamage` _returnvalue (`GameplayStatics.GetPlayerPawn` 0) (`self.Damage`) (`self.GetOwner`))
        (`/Game/Blueprints/Characters/Boss/BP_BossU.BossChargeTimeAfterHittingPlayer` (`self.Boss`))))
    (else
      (goto _label :!via `Reset`))))

(event `Reset Do Once`
  ;[1 0.1172 0] Hitting the player
  (goto _label :!via `Reset`))

(event `DisappearSword`
  (`self.SetActorHiddenInGame` true)
  (`self.SetActorEnableCollision` false))

(fn `UserConstructionScript`)