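; BP_Boss is a boss character that runs enemy waves behind a scalable shield, with state transitions and debug prints still in progress.
; At BeginPlay it sphere-traces for nearby spawn points, registers itself with each, and changes state after a delay.
; SpawnAWave triggers those spawners and starts a looping timer that counts actors tagged "Boss".
; A zero count reverses the shield timeline, changes state and starts the first-wave panic phase.
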(event `self.ReceiveBeginPlay`
  (`self.EnemySpawnerGraph_EventBeginPlay`)
  (`SceneComponent.SetRelativeScale3D` (`self.Shield`) (0.0 0.0 0.0))
  (set `self.BossState` "NewEnumerator2")
  (set `self.NextBossStateToSet` "NewEnumerator0")
  (`KismetSystemLibrary.Delay` 7.0)
  (`self.Spawn Enemies`))

(event `Set Boss State`
  (set `self.BossState` (`self.NextBossStateToSet`)))

(event `Camera Shake`
  (bind _returnvalue (`self.GetController` (`GameplayStatics.GetPlayerPawn` 0)))
  ;[1 0.3047 0] Camera Shake
  (`/Engine/EditorBlueprintResources/StandardMacros.IsValid` _returnvalue
    (:`Is Valid`
      (bind _asplayer_controller (cast `PlayerController` _returnvalue))
      (`PlayerController.ClientStartCameraShake` :`self` _asplayer_controller :`Shake` "/Game/Blueprints/CameraShakes/HeavyCameraShake.HeavyCameraShake_C"))))

(event `Grow Shield`
  (bind (_direction _lerp) (`Timeline|GrowShield` :!via `PlayFromStart` :!label _label)
    (:`Update`
      (`SceneComponent.SetRelativeScale3D` (`self.Shield`) (`KismetMathLibrary.VLerp` (0.0 0.0 0.0) (5.5 5.5 5.5) _lerp)))))

(event `DestroyShield`
  (goto _label :!via `ReverseFromEnd`))

(event `Spawn Enemies`
  (set `self.NextBossStateToSet` "NewEnumerator1")
  (`self.Set Boss State`))

(event `self.ReceiveTick`
  (params (DeltaSeconds :type "Float (single-precision)"))
  (`KismetSystemLibrary.PrintString` (`|GetEnumeratorNameAsString` (`self.BossState`))))

(event `Phase 1 Panic And Attack`
  (`KismetSystemLibrary.Delay` 4.0)
  (set `self.NextBossStateToSet` "NewEnumerator4"))

(event `Spawn Sword`
  (`KismetSystemLibrary.PrintString` "Gave Sword"))

(event `EnemySpawnerGraph_EventBeginPlay`
  (bind _returnvalue (`self.K2_GetActorLocation`))
  (bind _spawnercheckradius (`self.SpawnerCheckRadius`))
  ;[0.4297 1 0] Setup enemy spawn points and set boss reference in each of the spawner
  (bind _outhits (`KismetSystemLibrary.SphereTraceMultiForObjects` _returnvalue _returnvalue _spawnercheckradius (`|MakeArray` "ObjectTypeQuery1" "ObjectTypeQuery1" :!type "EObjectTypeQuery Enum") true))
  (`KismetSystemLibrary.DrawDebugSphere` _returnvalue _spawnercheckradius 12 (struct :`R` 0.150622 :`G` 1.0 :`A` 1.0) 5.0)
  (for _array_element _outhits
    (bind _asbp_boss_level_enemy_spawn_point (cast `/Game/Blueprints/EnemySpawnerSystem/BP_BossLevelEnemySpawnPoint` (`.HitActor` (`GameplayStatics.BreakHitResult` _array_element))))
    (`KismetArrayLibrary.Array_Add` (`self.SpawnerList`) _asbp_boss_level_enemy_spawn_point))
  (for _array_element_2 (`self.SpawnerList`)
    (set `/Game/Blueprints/EnemySpawnerSystem/BP_BossLevelEnemySpawnPoint.Boss` self _array_element_2)))

(event `CalculateNumberofSpawnedEnemies`
  (params (HowManyEnemiesSpawned :type Integer))
  ;[0 1 0.7188] Handled by Enemy Spawn Point
  (bind _output_get (set `self.NumberOfEnemies` (+ (`self.NumberOfEnemies`) HowManyEnemiesSpawned)))
  (`KismetSystemLibrary.PrintString` (`KismetStringLibrary.Concat_StrStr` (`KismetStringLibrary.Conv_IntToString` _output_get) " spawned in wave " (`KismetStringLibrary.Conv_IntToString` (`self.CurrentWave`)))))

(event `Spawn A Wave`
  ;[0.3828 0 1] Spawn A wave and start an event theat checks for the number of alive enemies
  (for _array_element (`self.SpawnerList`)
    (`/Game/Blueprints/EnemySpawnerSystem/BP_BossLevelEnemySpawnPoint.SpawnEnemy` _array_element))
  (`self.EnemySpawnCountCheck`)
  (bind _returnvalue (`KismetSystemLibrary.K2_SetTimerDelegate` (delegate `EnemySpawnCountCheck`) 1.0 true))
  (set `self.SpawnTimerHandle` _returnvalue))

(event `EnemySpawnCountCheck`
  (`|ExecutionSequence`
    (:`then_0`
      (bind _outactors (`GameplayStatics.GetAllActorsWithTag` "Boss"))
      (bind _returnvalue (`KismetArrayLibrary.Array_Length` _outactors))
      (if (== _returnvalue (`self.NumberOfEnemies`))
        (`KismetSystemLibrary.PrintString` "Nobody is ded")
        (else
          (bind _output_get (set `self.NumberOfEnemies` _returnvalue))
          (`KismetSystemLibrary.PrintString` (`KismetStringLibrary.Concat_StrStr` "Amount of peeps is: " (`KismetStringLibrary.Conv_IntToString` _output_get))))))
    (:`then_1`
      (if (== (`self.NumberOfEnemies`) 0)
        (`KismetSystemLibrary.K2_ClearAndInvalidateTimerHandle` (`self.SpawnTimerHandle`))
        (`self.DestroyShield`)
        (set `self.NextBossStateToSet` "NewEnumerator2")
        (`self.Set Boss State`)
        (switch `int` (`self.CurrentWave`)
          (:`Default`
            (`KismetSystemLibrary.PrintString` "SOMETHING IS WRONG BOi"))
          (:`0`
            (`self.Phase 1 Panic And Attack`)))))))

(fn `UserConstructionScript`)