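; BP_BossU is a wave-based boss with a shield, a gem weak point, a sword weapon and time-manipulation attacks.
; Nearby spawn points found by sphere trace spawn waves; a timer counts tagged enemies and, at zero, drops the shield and starts that wave's attack phase.
; Breaking the gem staggers the boss and swaps time, opening a timed crossbow window.
; A crossbow hit advances the wave; timeouts revert to the present and restart it.
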(event `self.ReceiveBeginPlay`
  (`|ExecutionSequence`
    (:`then_0`
      ;[0.125 1 0] Turn off Gem Collision
      (`PrimitiveComponent.SetCollisionEnabled` (`self.Box`) "NoCollision"))
    (:`then_1`
      ;[1 0 0.2812] Set starting boss states and init values
      (`self.EnemySpawnerGraph_EventBeginPlay`)
      (`SceneComponent.SetRelativeScale3D` (`self.Shield`) (0.0 0.0 0.0))
      (set `self.BossState` "NewEnumerator2")
      (set `self.NextBossStateToSet` "NewEnumerator0")
      (`KismetSystemLibrary.Delay` 7.0)
      (`self.Spawn Enemies`))
    (:`then_2`
      ;[0 1 0.3906] Set sword variable and boss variable in sword
      (bind _asbp_boss_weapon (cast `/Game/Blueprints/Characters/Boss/BP_BossWeapon` (`ChildActorComponent.ChildActor` (`self.Sword`))))
      (bind _output_get (set `self.Weapon` _asbp_boss_weapon))
      (set `/Game/Blueprints/Characters/Boss/BP_BossWeapon.Boss` self _output_get))
    (:`then_3`
      (`self.Update Boss Health`))))

(event `Set Boss State`
  ;[0 1 0.5547] Setting Boss Animation State
  (set `self.BossState` (`self.NextBossStateToSet`)))

(event `Camera Shake`
  (bind _returnvalue (`self.GetController` (`GameplayStatics.GetPlayerPawn` 0)))
  ;[1 0.3047 0] Camera Shake
  (`/Engine/EditorBlueprintResources/StandardMacros.IsValid` _returnvalue
    (:`Is Valid`
      (bind _asplayer_controller (cast `PlayerController` _returnvalue))
      (`PlayerController.ClientStartCameraShake` :`self` _asplayer_controller :`Shake` "/Game/Blueprints/CameraShakes/HeavyCameraShake.HeavyCameraShake_C"))))

(event `Grow Shield`
  ;[0.05469 0 1] Grow Shield and Destroy the shield
  (`self.ResetGem`)
  (bind (_direction _lerp) (`Timeline|GrowShield` :!via `PlayFromStart` :!label _label)
    (:`Update`
      (`SceneComponent.SetRelativeScale3D` (`self.Shield`) (`KismetMathLibrary.VLerp` (0.0 0.0 0.0) (5.5 5.5 5.5) _lerp)))))

(event `DestroyShield`
  ;[0.05469 0 1] Grow Shield and Destroy the shield
  (goto _label :!via `ReverseFromEnd`))

(event `self.ReceiveTick`
  (params (DeltaSeconds :type "Float (single-precision)"))
  (`KismetSystemLibrary.Delay` 2.0)
  (`KismetSystemLibrary.PrintString` (`|GetEnumeratorNameAsString` (`self.BossState`))))

(event `Spawn Enemies`
  ;[1 0.7969 0] Spawn Enemies First Wave
  (set `self.NextBossStateToSet` "NewEnumerator1")
  (`self.Set Boss State`))

(event `ResetGem`
  ;[1 0.8906 0] Reset gem collision and its Health
  (set `self.GemBroken?` false)
  (`PrimitiveComponent.SetCollisionEnabled` (`self.Box`) "NoCollision")
  (set `self.GemHealth` 100.0))

(event `BossChargeTimeAfterHittingPlayer`
  ;[0 0.6719 1] Charging Time Bubble
  (`/Game/Blueprints/Characters/Boss/BP_BossWeapon.Reset Do Once` (`self.Weapon`))
  (`/Game/Blueprints/Characters/Boss/BP_BossWeapon.DisappearSword` (`self.Weapon`))
  (`self.Set State` "NewEnumerator6")
  (bind (_direction _alpha) (`Timeline|GrowTimeBubble` :!via `PlayFromStart` :!label _label_2)
    (:`Update`
      (`SceneComponent.SetRelativeScale3D` (`self.TimeBubbleAttack`) (`KismetMathLibrary.VLerp` (0.0 0.0 0.0) (5.0 5.0 5.0) _alpha)))
    (:`Finished`
      ;[0.875 1 0] If player doesn't destroy the gem after the player is hit once, reverse time
      (if (not (`self.GemBroken?`))
        (`self.Reset And Start Previous Wave`)
        (else
          (goto _label_2 :!via `Stop`))))))

(event `BPSlowDownCharacter`
  ;[0 1 0.3906] Slow Down Boss
  (`/Game/Blueprints/Characters/Boss/BP_BossWeapon.Reset Do Once` (`self.Weapon`))
  (set `self.CustomTimeDilation` 0.2)
  (`KismetSystemLibrary.Delay` (`self.CharacterPrepTime`))
  (set `self.CustomTimeDilation` 1.0))

(event `BrokenGemStagger`
  ;[1 0 0.6797] Stagger
  (`/Engine/EditorBlueprintResources/StandardMacros.DoOnce` false :!label _label_3
    (:`Completed`
      (`|ExecutionSequence`
        (:`then_0`
          (set `self.GemBroken?` true))
        (:`then_1`
          (goto _label_2 :!via `Reverse`))
        (:`then_2`
          (`self.Set State` "NewEnumerator5")
          (bind _asbp_group_project_game_state (cast `/Game/Blueprints/GameFiles/BP_GroupProjectGameState` (`GameplayStatics.GetGameState`)))
          (`/Game/Blueprints/GameFiles/BP_GroupProjectGameState.SwapTime` _asbp_group_project_game_state))
        (:`then_3`
          (`Timeline|CountDown` :!via `PlayFromStart`
            (:`Finished`
              (if (not (`self.CrossBowHit?`))
                (`self.Reset And Start Previous Wave`))
              (set `self.CrossBowHit?` false))))))))

(event `Phase 1 Panic And Attack`
  ;[0 0.4844 1] Panic and Attack Phases
  (`PrimitiveComponent.SetCollisionEnabled` (`self.Box`) "QueryAndPhysics")
  (`KismetSystemLibrary.Delay` 4.0)
  (set `self.NextBossStateToSet` "NewEnumerator4")
  (goto _label_3 :!via `Reset`))

(event `Spawn Single Sword`
  ;[0 0.5547 1] Sword spawning and despawning
  ;;[0.125 1 0] Spawn Single Sword
  (`/Game/Blueprints/Characters/Boss/BP_BossWeapon.SpawnSingleSword` (`self.Weapon`)))

(event `Disappear Sword`
  ;[0 0.5547 1] Sword spawning and despawning
  ;;[1 0 0.9141] Disappear Single Sword
  (`/Game/Blueprints/Characters/Boss/BP_BossWeapon.DisappearSword` (`self.Weapon`)))

(event `DamageBoss`
  ;[0.4062 0 1] Actually Damage the boss with crossbow
  (set `self.CrossBowHit?` true)
  (if (> (- (`self.BossHealth`) 1) 0)
    (`/Engine/EditorBlueprintResources/StandardMacros.DecrementInt` (`self.BossHealth`)
      (:`  `
        (`self.Update Boss Health`)
        (`self.Start Next Wave`)))))

(event `Phase 2 Painc And Attack`
  ;[0 0.4844 1] Panic and Attack Phases
  (`PrimitiveComponent.SetCollisionEnabled` (`self.Box`) "QueryAndPhysics")
  (`KismetSystemLibrary.Delay` 4.0)
  (set `self.NextBossStateToSet` "NewEnumerator7")
  (goto _label_3 :!via `Reset`))

(event `Phase 3 Panic And Attack`
  ;[0 0.4844 1] Panic and Attack Phases
  (`PrimitiveComponent.SetCollisionEnabled` (`self.Box`) "QueryAndPhysics"))

(event `Spawn Tri Sword`
  ;[0 0.5547 1] Sword spawning and despawning
  ;;[1 0.09375 0] Spawn Tri Sword
  (`/Game/Blueprints/Characters/Boss/BP_BossWeapon.Spawn Tri Sword` (`self.Weapon`)))

(event `Phase 4 Panic And Attack`
  ;[0 0.4844 1] Panic and Attack Phases
  (`PrimitiveComponent.SetCollisionEnabled` (`self.Box`) "QueryAndPhysics"))

(event `Start Next Wave`
  ;[1 0 0.4687] Start the next wave
  (bind _result (`/Engine/EditorBlueprintResources/StandardMacros.IncrementInt` (`self.CurrentWave`))
    (:`  `
      (`self.Set State` "NewEnumerator2")
      (`KismetSystemLibrary.Delay` 5.0)
      (set `self.NextBossStateToSet` "NewEnumerator0")
      (`TextRenderComponent.K2_SetText` (`self.Wave Number Text`) (`KismetSystemLibrary.MakeLiteralText` (`KismetTextLibrary.Conv_StringToText` (`KismetStringLibrary.Concat_StrStr` "Wave: " (`KismetStringLibrary.Conv_IntToString` _result)))))
      (`KismetSystemLibrary.Delay` 2.0)
      (set `self.NextBossStateToSet` "NewEnumerator1"))))

(event `Reset And Start Previous Wave`
  ;[0.9453 1 0] Reset and start Previous Wave
  (`/Game/Blueprints/Xbow.LeaveXbow` (`self.XbowReference`))
  (bind _asbp_group_project_game_state (cast `/Game/Blueprints/GameFiles/BP_GroupProjectGameState` (`GameplayStatics.GetGameState`)))
  (`/Game/Blueprints/GameFiles/BP_GroupProjectGameState.ChangeEverythingToPresent` _asbp_group_project_game_state)
  (`self.Set State` "NewEnumerator2")
  (`KismetSystemLibrary.Delay` 5.0)
  (set `self.NextBossStateToSet` "NewEnumerator0")
  (`KismetSystemLibrary.Delay` 2.0)
  (set `self.NextBossStateToSet` "NewEnumerator1")
  (goto _label_3 :!via `Reset`))

(event `self.Box.OnComponentHit`
  (params (HitComponent :type "PrimitiveComponent Object Reference") (OtherActor :type "Actor Object Reference") (OtherComp :type "PrimitiveComponent Object Reference") (NormalImpulse :type "Vector Structure") (Hit :type "HitResult Structure (by ref)"))
  ;[0.1719 0 1] Take Gem Damage
  (`self.Take Damage` 5.0))

(event `Update Boss Health`
  ;[0 0.4375 1] Update Boss Health Text
  (`TextRenderComponent.K2_SetText` (`self.BHealthText`) (`KismetTextLibrary.Conv_IntToText` (`self.BossHealth`))))

(event `Take Damage`
  (params (Damage :type "Float (double-precision)"))
  (bind _newhealth (`/Game/Blueprints/CustomMacroLibraries/ML_HealthAndDamage.ReduceHealth` (`self.GemHealth`) Damage))
  ;[0.1719 0 1] Take Gem Damage
  (set `self.GemHealth` _newhealth)
  (if (`/Game/Blueprints/CustomMacroLibraries/ML_HealthAndDamage.HealthCheck` _newhealth)
    (`self.BrokenGemStagger`)
    (else
      (`KismetSystemLibrary.PrintString` "Damaged Gem"))))

(event `EnemySpawnerGraph_EventBeginPlay`
  (bind _returnvalue (`self.K2_GetActorLocation`))
  (bind _spawnercheckradius (`self.SpawnerCheckRadius`))
  ;[0.4297 1 0] Setup enemy spawn points and set boss reference in each of the spawner
  (bind _outhits (`KismetSystemLibrary.SphereTraceMultiForObjects` _returnvalue _returnvalue _spawnercheckradius (`|MakeArray` "ObjectTypeQuery1" "ObjectTypeQuery1" :!type "EObjectTypeQuery Enum") true))
  (`KismetSystemLibrary.DrawDebugSphere` _returnvalue _spawnercheckradius 12 (struct :`R` 0.150622 :`G` 1.0 :`A` 1.0) 5.0)
  (for _array_element _outhits
    (bind _asbp_boss_level_enemy_spawn_point (cast `/Game/Blueprints/EnemySpawnerSystem/BP_BossLevelEnemySpawnPoint` (`.HitActor` (`GameplayStatics.BreakHitResult` _array_element))))
    (`KismetArrayLibrary.Array_Add` (`self.SpawnerList`) _asbp_boss_level_enemy_spawn_point))
  (for _array_element_2 (`self.SpawnerList`)
    (set `/Game/Blueprints/EnemySpawnerSystem/BP_BossLevelEnemySpawnPoint.Boss` self _array_element_2)))

(event `CalculateNumberofSpawnedEnemies`
  (params (HowManyEnemiesSpawned :type Integer))
  ;[0 1 0.7188] Handled by Enemy Spawn Point
  (bind _output_get (set `self.NumberOfEnemies` (+ (`self.NumberOfEnemies`) HowManyEnemiesSpawned)))
  (`KismetSystemLibrary.PrintString` (`KismetStringLibrary.Concat_StrStr` (`KismetStringLibrary.Conv_IntToString` _output_get) " spawned in wave " (`KismetStringLibrary.Conv_IntToString` (`self.CurrentWave`)))))

(event `Spawn A Wave`
  ;[0.3828 0 1] Spawn A wave and start an event theat checks for the number of alive enemies
  (for _array_element (`self.SpawnerList`)
    (`/Game/Blueprints/EnemySpawnerSystem/BP_BossLevelEnemySpawnPoint.SpawnEnemy` _array_element))
  (`self.EnemySpawnCountCheck`)
  (bind _returnvalue (`KismetSystemLibrary.K2_SetTimerDelegate` (delegate `EnemySpawnCountCheck`) 1.0 true))
  (set `self.SpawnTimerHandle` _returnvalue))

(event `EnemySpawnCountCheck`
  (`|ExecutionSequence`
    (:`then_0`
      (bind _outactors (`GameplayStatics.GetAllActorsWithTag` "Boss"))
      (bind _returnvalue (`KismetArrayLibrary.Array_Length` _outactors))
      (if (== _returnvalue (`self.NumberOfEnemies`))
        (`KismetSystemLibrary.PrintString` "Nobody is ded")
        (else
          (bind _output_get (set `self.NumberOfEnemies` _returnvalue))
          (`KismetSystemLibrary.PrintString` (`KismetStringLibrary.Concat_StrStr` "Amount of peeps is: " (`KismetStringLibrary.Conv_IntToString` _output_get))))))
    (:`then_1`
      (if (== (`self.NumberOfEnemies`) 0)
        (`KismetSystemLibrary.K2_ClearAndInvalidateTimerHandle` (`self.SpawnTimerHandle`))
        (`self.DestroyShield`)
        (set `self.NextBossStateToSet` "NewEnumerator2")
        (`self.Set Boss State`)
        (switch `int` (`self.CurrentWave`)
          (:`Default`
            (`KismetSystemLibrary.PrintString` "SOMETHING IS WRONG BOi"))
          (:`0`
            (`self.Phase 1 Panic And Attack`))
          (:`1`
            (`self.Phase 2 Painc And Attack`))
          (:`2`
            (`self.Phase 3 Panic And Attack`))
          (:`3`
            (`self.Phase 4 Panic And Attack`)))))))

(fn `UserConstructionScript`)