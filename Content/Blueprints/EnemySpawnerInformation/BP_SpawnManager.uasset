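; Wave-based combat manager that collects BP_EnemySpawnPoint actors within a radius on BeginPlay and registers itself with each.
; StartCombat spawns the first wave through those points and starts a looping timer that polls the enemy count, which CalculateNumberofSpawnedEnemies increases.
; At zero enemies it waits that wave's delay, then spawns the next through a DoOnce reset per wave, or prints "Combat Over" after the last.
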(event `self.ReceiveBeginPlay`
  (bind _returnvalue (`self.K2_GetActorLocation`))
  (bind _spawnercheckradius (`self.SpawnerCheckRadius`))
  ;[0 0.3437 1] Get all enemy spawn points in a user defined radius and setup the spawn manager variable in each one of them
  (bind _outactors (`KismetSystemLibrary.SphereOverlapActors` _returnvalue _spawnercheckradius (`|MakeArray` "ObjectTypeQuery2" :!type "EObjectTypeQuery Enum") "/Game/Blueprints/EnemySpawnerInformation/BP_EnemySpawnPoint.BP_EnemySpawnPoint_C"))
  (`KismetSystemLibrary.DrawDebugSphere` _returnvalue _spawnercheckradius 12 (struct :`R` 0.150622 :`G` 1.0 :`A` 1.0) 5.0)
  (for _array_element _outactors
    (bind _asbp_enemy_spawn_point (cast `/Game/Blueprints/EnemySpawnerInformation/BP_EnemySpawnPoint` _array_element))
    (`KismetArrayLibrary.Array_AddUnique` (`self.SpawnerList`) _asbp_enemy_spawn_point))
  (for _array_element_2 (`self.SpawnerList`)
    (set `/Game/Blueprints/EnemySpawnerInformation/BP_EnemySpawnPoint.SpawnManager` self _array_element_2)))

(event `Start Combat`
  ;[0 0.7422 1] Spawn the first wave and start off a custom tick
  (`self.Spawn A Wave`)
  (`self.EnemyCountChecker`)
  (`KismetSystemLibrary.K2_SetTimerDelegate` (delegate `EnemyCountChecker`) 2.0 true))

(event `Spawn A Wave`
  ;[0.1953 1 0] Spawn Points Spawn enemies Based On a condition(Mostly after clearing out a wave)
  (set `self.CurrentWaveNumber` (+ (`self.CurrentWaveNumber`) 1))
  (for _array_element (`self.SpawnerList`)
    (`/Game/Blueprints/EnemySpawnerInformation/BP_EnemySpawnPoint.SpawnEnemy` _array_element))
  (`self.Reset Do Once`))

(event `EnemyCountChecker`
  ;[0 0.8594 1] Every two seconds check if the enemy count is zero, if it is do the wave delay and spawn the next wave. If all the waves have been spawmed, finish combat
  (if (== (`self.NumberOfEnemies`) 0)
    (`KismetSystemLibrary.Delay` (`|GetArrayItem` (`self.WaitBetweenWaves`) (`self.CurrentWaveNumber`)))
    (if (not (> (+ (`self.CurrentWaveNumber`) 1) (`self.MaxWaveNumber`)))
      (`/Engine/EditorBlueprintResources/StandardMacros.DoOnce` false :!label _label
        (:`Completed`
          (`self.Spawn A Wave`)))
      (else
        (`KismetSystemLibrary.PrintString` "Combat Over")))))

(event `Reset Do Once`
  ;[0 0.8594 1] Every two seconds check if the enemy count is zero, if it is do the wave delay and spawn the next wave. If all the waves have been spawmed, finish combat
  (goto _label :!via `Reset`))

(event `CalculateNumberofSpawnedEnemies`
  (params (HowManyEnemiesSpawned :type Integer))
  ;[1 0 0.07031] Caluclate the number of enemies spawned in the wave
  (bind _output_get (set `self.NumberOfEnemies` (+ (`self.NumberOfEnemies`) HowManyEnemiesSpawned)))
  (`KismetSystemLibrary.PrintString` (`KismetStringLibrary.Concat_StrStr` (`KismetStringLibrary.Conv_IntToString` _output_get) " spawned in wave " (`KismetStringLibrary.Conv_IntToString` (`self.CurrentWaveNumber`)))))

(fn `CalculateEnemyNumber`)

(fn `UserConstructionScript`)